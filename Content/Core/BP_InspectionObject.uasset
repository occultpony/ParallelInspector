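; Inspection item that rides a conveyor to a stop, can be grabbed, then rides off to be destroyed.
; Construction script sets it up by Type; non-normal items get at least one randomly broken trait among mass, buoyancy, electricity and impact sound.
; Tick moves it and scrolls the belt material; Interact toggles grabbing through the player controller.
; Impact and water sounds reflect weight, and GoAway adds a static-noise glitch to non-normal items.
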(event Interact(BP_InteractionComp)
  (bind _returnvalue (Game|GetPlayerController 0))
  (bind _output_get (Variables|Default|SetbGrabbed (not (Variables|Default|GetbGrabbed))))
  (if _output_get
    (Variables|Default|SetbInDestination true)
    (Class|BIPIGame|StartGrabbing(Message) _returnvalue self)
    (else
      (Class|BIPIGame|StopGrabbing(Message) _returnvalue))))

(event OnComponentBeginOverlap(StaticMesh)
  (params (OverlappedComponent :type Primitive%20Component%20Object%20Reference) (OtherActor :type Actor%20Object%20Reference) (OtherComp :type Primitive%20Component%20Object%20Reference) (OtherBodyIndex :type Integer) (bFromSweep :type Boolean) (SweepResult :type Hit%20Result%20Structure%20%28by%20ref%29))
  (bind (_soundvar _isheavy) (CallFunction|GetIsHeavy))
  (bind _returnvalue (Transformation|GetActorLocation))
  (Utilities|Casting|CastToWaterBody OtherActor)
  (if (Utilities|IsValid (Variables|Default|GetEditableBuoyancy))
    (if _isheavy
      (Audio|PlaySoundatLocation "/Game/Sounds/S_Water_Ripple.S_Water_Ripple" _returnvalue "0, 0, 0" 1.0 1.0 0.0 0 0 0 0)
      (else
        (bind _returnvalue_2 (Audio|SpawnSoundatLocation "/Game/Sounds/S_Water_Plunge.S_Water_Plunge" _returnvalue "0, 0, 0" 1.0 1.0 0.0 0 0 :!label _label))
        (Effects|Components|ParticleSystem|SetIntParameter _returnvalue_2 "Heavy" _soundvar)))
    (else
      (goto _label))))

(event OnComponentEndOverlap(StaticMesh)
  (params (OverlappedComponent :type Primitive%20Component%20Object%20Reference) (OtherActor :type Actor%20Object%20Reference) (OtherComp :type Primitive%20Component%20Object%20Reference) (OtherBodyIndex :type Integer))
  (Utilities|Casting|CastToWaterBody OtherActor))

(event Custom|GoAway
  (bind _staticmesh (Variables|Default|GetStaticMesh))
  (Class|BIPIGame|StopGrabbing(Message) (Game|GetPlayerController 0))
  (Variables|Default|SetbGrabbed false)
  (Transformation|SetActorTransform (Math|Transform|MakeTransform "280.000000,0.000000,200.000000" "0, 0, 0" "1.000000,1.000000,1.000000"))
  (Physics|SetSimulatePhysics (Variables|Default|GetStaticMesh) false)
  (Variables|Default|SetbAboutToBeDestroyed true)
  (Variables|Default|SetbInDestination false)
  (Components|DestroyComponent (Variables|Default|GetBP_InteractionComp))
  (if (not (Variables|Default|GetbIsNormal))
    (bind _returnvalue (Rendering|Material|CreateDynamicMaterialInstance _staticmesh 0 (Rendering|Material|GetMaterial _staticmesh 0) "None" :!class /Script/Engine.PrimitiveComponent))
    (bind _output_get (Variables|Default|SetMat _returnvalue))
    (Rendering|Material|SetScalarParameterValue _output_get "Noise" 0.7 :!class /Script/Engine.MaterialInstanceDynamic)
    (Utilities|Time|SetTimerbyEvent (delegate Custom|CustomEvent) (Math|Random|RandomFloatinRange 0.3 1.0))
    (Audio|PlaySoundatLocation "/Game/Sounds/WhiteNoise_Modulated.WhiteNoise_Modulated" (Transformation|GetActorLocation) "0, 0, 0" 1.0 1.0 0.0 0 0 0 0)))

(event Custom|CustomEvent
  (Rendering|Material|SetScalarParameterValue (Variables|Default|GetMat) "Noise" 0.9 :!class /Script/Engine.MaterialInstanceDynamic)
  (Audio|PlaySoundatLocation "/Game/Sounds/WhiteNoise_Modulated.WhiteNoise_Modulated" (Transformation|GetActorLocation) "0, 0, 0" 1.0 1.0 0.0 0 0 0 0)
  (Utilities|FlowControl|Delay 0.2)
  (Rendering|Material|SetScalarParameterValue (Variables|Default|GetMat) "Noise" (Math|Random|RandomFloatinRange 0.0 0.3) :!class /Script/Engine.MaterialInstanceDynamic))

(event EventBeginPlay
  (Variables|Default|SetbInDestination false))

(event Collision|EventHit
  (params (MyComp :type Primitive%20Component%20Object%20Reference) (Other :type Actor%20Object%20Reference) (OtherComp :type Primitive%20Component%20Object%20Reference) (bSelfMoved :type Boolean) (HitLocation :type Vector :default "0, 0, 0") (HitNormal :type Vector :default "0, 0, 0") (NormalImpulse :type Vector :default "0, 0, 0") (Hit :type Hit%20Result%20Structure%20%28by%20ref%29))
  (bind _sound (Variables|Default|GetSound))
  (bind _duration (Variables|/Script/Engine.SoundBase|GetDuration _sound))
  (if (Variables|Default|GetbInDestination)
    (Utilities|FlowControl|DoOnce false :!label _label
      (:Completed
        (bind _returnvalue (Audio|SpawnSoundatLocation _sound HitLocation "0, 0, 0" (Math|Float|MapRangeClamped (Math|Vector|VectorLength (Math|Conversions|ToVector(Float) (.x (Transformation|GetComponentVelocity (Variables|Default|GetStaticMesh))))) 25.0 5e+01 0.0 1.0) 1.0 0.0 0 0))
        (Effects|Components|ParticleSystem|SetIntParameter _returnvalue "Heavy" (.SoundVar (CallFunction|GetIsHeavy)))
        (Utilities|FlowControl|Delay (Math|Random|RandomFloatinRange (/ _duration 2.0) _duration))
        (goto _label Reset)))))

(event EventTick
  (params (DeltaSeconds :type Float%20%28single-precision%29))
  (bind _returnvalue (Transformation|GetActorLocation))
  (if (Variables|Default|GetbGrabbed)
    (Class|BIPIGame|UpdateGrabbing(Message) (Game|GetPlayerController 0) self)
    (elif (not (Variables|Default|GetbInDestination))
      (Transformation|AddActorWorldOffset (Math|Vector|MakeVector 0.0 (* DeltaSeconds 2.5e+02) 0.0))
      (bind _returnvalue_2 (Rendering|Material|CreateDynamicMaterialInstance (Variables|/Script/Engine.StaticMeshActor|GetStaticMeshComponent (Variables|Default|GetBelt)) 0 "/Game/Environment/M_Belt.M_Belt" "None" :!class /Script/Engine.PrimitiveComponent))
      (Rendering|Material|SetScalarParameterValue _returnvalue_2 "Offset" (- -4.5e+02 (.y _returnvalue)) :!class /Script/Engine.MaterialInstanceDynamic)
      (if (Math|Float|NearlyEqual(Float) (.y _returnvalue) (Math|Float|SelectFloat 4.5e+02 0.0 (Variables|Default|GetbAboutToBeDestroyed)) 5.0)
        (Variables|Default|SetbInDestination true)
        (if (Variables|Default|GetbAboutToBeDestroyed)
          (Actor|DestroyActor))))))

(fn ConstructionScript
  (bind _array (Utilities|Array|MakeArray "/Game/Sounds/S_RubberDuck_Fall.S_RubberDuck_Fall" "/Game/Sounds/S_Bolt_Fall.S_Bolt_Fall" "/Game/Sounds/S_CinderBlock_Fall.S_CinderBlock_Fall" "/Game/Sounds/S_Pear_Fall.S_Pear_Fall" "/Game/Sounds/S_PongBall_Fall.S_PongBall_Fall" "/Engine/VREditor/Sounds/VR_click1_Cue.VR_click1_Cue" "/Game/Sounds/S_Weird_Fall.S_Weird_Fall"))
  (bind _type (Variables|Default|GetType))
  (bind _staticmesh (Variables|Default|GetStaticMesh))
  (bind _normalproperties (Variables|Default|GetNormalProperties))
  (bind _value (Utilities|Map|Find _normalproperties _type))
  (bind _massmax (Variables|/Game/Core/DA_NormalProperties.DA_NormalProperties_C|GetMassMax _value))
  (bind _massmin (Variables|/Game/Core/DA_NormalProperties.DA_NormalProperties_C|GetMassMin _value))
  (Components|StaticMesh|SetStaticMesh _staticmesh (.Value (Utilities|Map|Find (Variables|Default|GetMeshes) _type)))
  (Rendering|Material|SetMaterial _staticmesh 0 (.OutItem (Utilities|Array|Random (Variables|/Game/Core/DA_NormalProperties.DA_NormalProperties_C|GetMaterials _value))))
  (LocalVariables|SetNormalPrope (Variables|/Game/Core/DA_NormalProperties.DA_NormalProperties_C|GetProperties _value))
  (if (Variables|Default|GetbIsNormal)
    (bind _output_get (LocalVariables|SetMass (Math|Random|RandomFloatinRange (Variables|/Game/Core/DA_NormalProperties.DA_NormalProperties_C|GetMassMin _value) (Variables|/Game/Core/DA_NormalProperties.DA_NormalProperties_C|GetMassMax _value))))
    (Class|PrimitiveComponent|SetMassOverrideinKg (Variables|Default|GetStaticMesh) "None" _output_get true)
    (if (.bItDrowns (Utilities|Struct|BreakSObjectProperties (LocalVariables|GetNormalPrope)))
      (Components|DestroyComponent (Variables|Default|GetEditableBuoyancy))
      (else
        (Class|EditableBuoyancyComponent|SetBuoyancyCoefficient (Variables|Default|GetEditableBuoyancy) (LocalVariables|GetMass))))
    (Variables|Default|SetbElectric (.bElectric (Utilities|Struct|BreakSObjectProperties (LocalVariables|GetNormalPrope))))
    (Variables|Default|SetSound (Variables|/Game/Core/DA_NormalProperties.DA_NormalProperties_C|GetSound _value))
    (else
      (LocalVariables|SetBrokenPropertyIndex (Math|Random|RandomIntegerinRange 0 3))
      (bind _output_get_2 (LocalVariables|SetMass (Math|Float|SelectFloat (CallFunction|RandomFloatExcludingRange _massmin _massmax) (Math|Random|RandomFloatinRange _massmin _massmax) (or (== (LocalVariables|GetBrokenPropertyIndex) 0) (Math|Random|RandomBoolwithWeight 0.1)))))
      (Class|PrimitiveComponent|SetMassOverrideinKg (Variables|Default|GetStaticMesh) "None" _output_get_2 true)
      (if (select (or (== (LocalVariables|GetBrokenPropertyIndex) 1) (Math|Random|RandomBoolwithWeight 0.1)) (not (.bItDrowns (Utilities|Struct|BreakSObjectProperties (LocalVariables|GetNormalPrope)))) (.bItDrowns (Utilities|Struct|BreakSObjectProperties (LocalVariables|GetNormalPrope))))
        (Components|DestroyComponent (Variables|Default|GetEditableBuoyancy))
        (elif (.bItDrowns (Utilities|Struct|BreakSObjectProperties (LocalVariables|GetNormalPrope)))
          (Class|EditableBuoyancyComponent|SetBuoyancyCoefficient (Variables|Default|GetEditableBuoyancy) (LocalVariables|GetMass))))
      (Variables|Default|SetbElectric (select (or (== (LocalVariables|GetBrokenPropertyIndex) 2) (Math|Random|RandomBoolwithWeight 0.1)) (not (.bElectric (Utilities|Struct|BreakSObjectProperties (LocalVariables|GetNormalPrope)))) (.bElectric (Utilities|Struct|BreakSObjectProperties (LocalVariables|GetNormalPrope)))))
      (Utilities|Array|RemoveItem _array (Variables|/Game/Core/DA_NormalProperties.DA_NormalProperties_C|GetSound _value))
      (Variables|Default|SetSound (select (or (== (LocalVariables|GetBrokenPropertyIndex) 3) (Math|Random|RandomBoolwithWeight 0.1)) (.OutItem (Utilities|Array|Random _array)) (Variables|/Game/Core/DA_NormalProperties.DA_NormalProperties_C|GetSound _value))))))

(fn RandomFloatExcludingRange
  (params (Min :type Float%20%28double-precision%29) (Max :type Float%20%28double-precision%29))
  (bind _output_get (LocalVariables|SetRandom (Math|Random|RandomFloatinRange 0.0 1e+02) :!label _label))
  (if (Math|Float|InRange(Float) _output_get (* Min 0.5) (* Max 1.5))
    (goto _label)
    (else
      (return (LocalVariables|GetRandom)))))

(fn GetIsHeavy
  (bind _type (Variables|Default|GetType))
  (bind _normalproperties (Variables|Default|GetNormalProperties))
  (bind _staticmesh (Variables|Default|GetStaticMesh))
  (bind _returnvalue (Physics|GetMass _staticmesh))
  (bind _value (Utilities|Map|Find _normalproperties _type))
  (bind _massmax (Variables|/Game/Core/DA_NormalProperties.DA_NormalProperties_C|GetMassMax _value))
  (bind _massmin (Variables|/Game/Core/DA_NormalProperties.DA_NormalProperties_C|GetMassMin _value))
  (bind _returnvalue_2 (* _massmin 0.5))
  (bind _returnvalue_3 (> _massmin 1e+01))
  (bind _returnvalue_4 (* _massmax 1.5))
  (bind _returnvalue_5 (> _returnvalue _returnvalue_4))
  (bind _returnvalue_6 (> _returnvalue _returnvalue_2))
  (bind _returnvalue_7 (select _returnvalue_3 _returnvalue_6 _returnvalue_5))
  (return (Math|Integer|SelectInt 1 0 _returnvalue_7) _returnvalue_7))