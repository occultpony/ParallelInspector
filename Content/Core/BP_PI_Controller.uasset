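; Player controller that handles interaction, physics-based grabbing and game input for approving or rejecting objects.
; Tick traces from the camera, ignoring the last target's owner, to find BP_InteractionComp and show its prompt; the prompt-clearing nodes are disconnected.
; Keys call interaction, quit, or send start, approve and reject messages to the game mode.
; Grab events drive the pawn's PhysicsHandle, with UpdateGrabbing placing its target along the view at a fraction of trace distance.
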(event EventStartGrabbing
  (params (SelfRef :type BP%20Inspection%20Object%20Object%20Reference))
  (Physics|Components|PhysicsHandle|GrabComponentatLocationwithRotation (Variables|Default|GetPlayerHandle) (Variables|/Game/Core/BP_InspectionObject.BP_InspectionObject_C|GetStaticMesh SelfRef) "None" (Transformation|GetActorLocation SelfRef) "0, 0, 0")
  (Variables|Default|SetbGrabbing true))

(event EventStopGrabbing
  (Physics|Components|PhysicsHandle|ReleaseComponent (Variables|Default|GetPlayerHandle))
  (Variables|Default|SetbGrabbing false))

(event EventBeginPlay
  (Variables|Default|SetbGameGoes false)
  (Variables|Default|SetPlayerHandle (Actor|GetComponentbyClass (Game|Player|GetPlayerPawn 0) "/Script/Engine.PhysicsHandleComponent")))

(event EventTick
  (params (DeltaSeconds :type Float%20%28single-precision%29))
  (bind _returnvalue (Game|GetPlayerCameraManager 0))
  (bind _returnvalue_2 (Camera|GetCameraLocation _returnvalue))
  (if (Utilities|IsValid (Variables|Default|GetInteractableComp))
    (Variables|Default|SetNewVar (Utilities|Array|MakeArray (Components|GetOwner (Variables|Default|GetInteractableComp))))
    (else
      (Variables|Default|SetNewVar (Utilities|Array|MakeArray 0))))
  (bind (_outhit _returnvalue_3) (Collision|LineTraceByChannel _returnvalue_2 (+ _returnvalue_2 (* (Math|Vector|GetForwardVector (Camera|GetCameraRotation _returnvalue)) 7e+02)) "TraceTypeQuery1" false (Variables|Default|GetNewVar) "ForOneFrame"))
  (if _returnvalue_3
    (Variables|Default|SetTraceLength (Math|Vector|VectorLength (- (.location _outhit) (.tracestart _outhit))))
    (if (Utilities|IsValid (.hitactor _outhit))
      (if (Utilities|IsValid (Actor|GetComponentbyClass (.hitactor _outhit) "/Game/Core/BP_InteractionComp.BP_InteractionComp_C"))
        (bind _output_get (Variables|Default|SetInteractableComp (Actor|GetComponentbyClass (.hitactor _outhit) "/Game/Core/BP_InteractionComp.BP_InteractionComp_C")))
        (Class|BIPIGame|UpdateInteractionPrompt(Message) (Game|GetGameMode) (Variables|/Game/Core/BP_InteractionComp.BP_InteractionComp_C|GetInteractionName _output_get) true))
      (elif (Variables|Default|GetbGrabbing)
        _))))

(event EventUpdateGrabbing
  (params (SelfRef :type Actor%20Object%20Reference))
  (bind _returnvalue (Game|GetPlayerCameraManager 0))
  (bind _tracelength (Variables|Default|GetTraceLength))
  (Physics|Components|PhysicsHandle|SetTargetLocation (Variables|Default|GetPlayerHandle) (+ (Transformation|GetWorldLocation (Variables|/Script/Engine.PlayerCameraManager|GetTransformComponent _returnvalue)) (* (Math|Vector|GetForwardVector (Camera|GetCameraRotation _returnvalue)) (* _tracelength 0.7))))
  (Development|PrintString (Utilities|String|ToString(Float) _tracelength) true true "(R=0.000000,G=0.660000,B=1.000000,A=1.000000)" 0.0))

(event EventGameFinished
  (Variables|Default|SetbGameGoes false))

(event Input|KeyboardEvents|Enter
  (params (Key :type Key%20Structure))
  (:Pressed
    (if (not (Variables|Default|GetbGameGoes))
      (Variables|Default|SetbGameGoes true)
      (Class|BIPIGame|StartGame(Message) (Game|GetGameMode)))))

(event Input|KeyboardEvents|E
  (params (Key :type Key%20Structure))
  (:Pressed
    (bind _interactablecomp (Variables|Default|GetInteractableComp)
      (:then
        (Default|CallInteract _interactablecomp))
      (:else))))

(event Input|KeyboardEvents|Q
  (params (Key :type Key%20Structure))
  (:Pressed
    (Class|BIPIGame|RejectObject(Message) (Game|GetGameMode))))

(event Input|KeyboardEvents|W
  (params (Key :type Key%20Structure))
  (:Pressed
    (Class|BIPIGame|ApproveObject(Message) (Game|GetGameMode))))

(event Input|KeyboardEvents|Escape
  (params (Key :type Key%20Structure))
  (:Pressed
    (Game|QuitGame 0 "Quit" false)))

(fn ConstructionScript)