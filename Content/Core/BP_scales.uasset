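; BP_scales is a scale actor that shows the combined mass of static mesh components overlapping its Weighter component.
; On begin overlap it adds the mesh to a tracked list, re-sums the masses and writes the total, rounded to two decimals, as kilograms to a text render.
; On end overlap it removes the mesh and shows a blank placeholder instead of recomputing the remaining total.
; Both overlap events also print the component's name.
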(event OnComponentBeginOverlap(Weighter)
  (params (OverlappedComponent :type Primitive%20Component%20Object%20Reference) (OtherActor :type Actor%20Object%20Reference) (OtherComp :type Primitive%20Component%20Object%20Reference) (OtherBodyIndex :type Integer) (bFromSweep :type Boolean) (SweepResult :type Hit%20Result%20Structure%20%28by%20ref%29))
  (bind _wightedcomps (Variables|Default|GetWightedComps))
  (Development|PrintString (Utilities|GetDisplayName OtherComp))
  (bind _asstatic_mesh_component (Utilities|Casting|CastToStaticMeshComponent OtherComp))
  (Utilities|Array|Add _wightedcomps _asstatic_mesh_component)
  (Variables|Default|SetTotalWeight 0.0)
  (for _array_element _wightedcomps
    (Variables|Default|SetTotalWeight (+ (Variables|Default|GetTotalWeight) (Physics|GetMass _array_element))))
  (Rendering|Components|TextRender|SetText (Variables|Default|GetTextRender) (Utilities|Text|FormatText "{mass} kg" (* (Math|Float|Round (* (Variables|Default|GetTotalWeight) 1e+02)) 0.01))))

(event OnComponentEndOverlap(Weighter)
  (params (OverlappedComponent :type Primitive%20Component%20Object%20Reference) (OtherActor :type Actor%20Object%20Reference) (OtherComp :type Primitive%20Component%20Object%20Reference) (OtherBodyIndex :type Integer))
  (Development|PrintString (Utilities|GetDisplayName OtherComp))
  (bind _asstatic_mesh_component (Utilities|Casting|CastToStaticMeshComponent OtherComp))
  (Utilities|Array|RemoveItem (Variables|Default|GetWightedComps) _asstatic_mesh_component)
  (Rendering|Components|TextRender|SetText (Variables|Default|GetTextRender) (Utilities|Text|FormatText "---.-- kg")))

(fn ConstructionScript)